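; Player Blueprint for a physics ball that is charged and launched in the camera's yaw direction.
; Mouse axes steer the controller, and Tick keeps the spring arm just above the sphere.
; Holding left mouse builds LaunchSpeed over time and releasing zeroes it, while Space applies it as linear velocity.
; Launching requires a near-stationary sphere, which Tick snaps to a full stop, printing speed and launch state for debugging.
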(event EventTick
  (params (DeltaSeconds :type Float%20%28single-precision%29))
  (bind _sphere (Variables|Default|GetSphere))
  (bind _returnvalue (Transformation|GetComponentVelocity _sphere))
  (bind _returnvalue_2 (Math|Vector|VectorLength _returnvalue))
  (Transformation|SetWorldLocation (Variables|Default|GetSpringArm) (+ (Transformation|GetWorldLocation (Variables|Default|GetSphere)) "0.000000,0.000000,40.000000") false false)
  (if (Variables|Default|GetisCharging)
    (bind _output_get (Variables|Default|SetLaunchSpeed (+ (* DeltaSeconds 1.5e+03) (Variables|Default|GetLaunchSpeed)))))
  (Development|PrintString (Utilities|String|ToString(Float) _output_get) true true "(R=0.000000,G=0.660000,B=1.000000,A=1.000000)" 0.0)
  (Development|PrintString (Utilities|String|ToString(Boolean) (Variables|Default|GetcanLaunch)) true true "(R=0.000000,G=0.660000,B=1.000000,A=1.000000)" 0.0)
  (Development|PrintString (Utilities|String|ToString(Float) _returnvalue_2) true true "(R=0.000000,G=0.660000,B=1.000000,A=1.000000)" 0.0)
  (if (<= _returnvalue_2 0.1)
    (Variables|Default|SetcanLaunch true)
    (else
      (Variables|Default|SetcanLaunch false)))
  (if (<= (Math|Vector|VectorLength (Transformation|GetComponentVelocity (Variables|Default|GetSphere))) 0.1)
    (Physics|SetPhysicsLinearVelocity (Variables|Default|GetSphere) "0, 0, 0" false "None")))

(event Input|MouseEvents|MouseX
  (params (AxisValue :type Float%20%28single-precision%29))
  (Pawn|Input|AddControllerYawInput AxisValue))

(event Input|MouseEvents|MouseY
  (params (AxisValue :type Float%20%28single-precision%29))
  (Pawn|Input|AddControllerPitchInput (* AxisValue -1.0)))

(event Input|MouseEvents|LeftMouseButton
  (params (Key :type Key%20Structure :default "None"))
  (:Pressed
    (Variables|Default|SetisCharging true))
  (:Released
    (Variables|Default|SetisCharging false)
    (Variables|Default|SetLaunchSpeed 0.0)))

(event Input|KeyboardEvents|SpaceBar
  (params (Key :type Key%20Structure :default "None"))
  (:Pressed
    (if (Variables|Default|GetcanLaunch)
      (Physics|SetPhysicsLinearVelocity (Variables|Default|GetSphere) (* (Math|Vector|GetForwardVector (Math|Rotator|MakeRotator 0.0 0.0 (.Yaw (Math|Rotator|BreakRotator (Pawn|GetControlRotation :!class /Script/Engine.Pawn))))) (Variables|Default|GetLaunchSpeed)) false "None")
      (Variables|Default|SetcanLaunch false))))

(fn ConstructionScript)